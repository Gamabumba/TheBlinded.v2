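; Player character Blueprint, named as a cameraless variant, that plays an attack animation on input.
; The Attack input press calls an Attack event, which only forwards to AttackEffects.
; AttackEffects plays the attack montage at a rate set by AttackSpeed, with no hit or damage logic in this graph.
; BeginPlay, overlap and Tick are disabled stubs, and the construction script only calls its parent.
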(event `InputAction|Attack`
  (params (Key :type "Key Structure"))
  (:`Pressed`
    (`self.Attack`)))

(event `Attack`
  (`self.AttackEffects`))

(event `AttackEffects`
  (`self.PlayAnimMontage` "/Game/Player/Characters/ExtendedY-bot/Animations/AM_Attck.AM_Attck" (`self.AttackSpeed`)))

(fn `UserConstructionScript`
  (`parent.UserConstructionScript`))