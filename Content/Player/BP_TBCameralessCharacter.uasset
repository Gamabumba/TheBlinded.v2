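; BP_TBCameralessCharacter is a player character Blueprint that turns its mesh to face the mouse cursor while alive.
; Each Tick, if HealthComponent is not dead, it traces under player 0's cursor against WorldStatic objects and applies the look-at yaw to the mesh with a fixed offset.
; Only the mesh rotates, with pitch and roll held at zero; a disconnected SetActorRotation alternative never runs.
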(event `self.ReceiveTick`
  (params (DeltaSeconds :type "Float (single-precision)"))
  (bind (_returnvalue_roll _returnvalue_pitch _returnvalue_yaw) (`KismetMathLibrary.BreakRotator` (`KismetMathLibrary.FindLookAtRotation` (`self.K2_GetActorLocation`) (`.ImpactPoint` (`GameplayStatics.BreakHitResult` (`PlayerController.GetHitResultUnderCursorForObjects` (`GameplayStatics.GetPlayerController` 0) (`|MakeArray` "ObjectTypeQuery1" :!type "EObjectTypeQuery Enum") true))))))
  (if (not (`TBHealthComponent.IsDead` (`self.HealthComponent`)))
    (`SceneComponent.K2_SetWorldRotation` (`self.Mesh`) (`KismetMathLibrary.MakeRotator` 0.0 0.0 (+ _returnvalue_yaw -110.0)) false false)))

(fn `UserConstructionScript`)