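; Player character Blueprint that handles a sword attack from the Attack input.
; A macro gates attacks on IsAttack, then AttackEffects plays the attack montage at AttackSpeed and clears the flag after its scaled duration.
; LaunchAttack, not called within this graph, line-traces forward for Pawns with debug drawing and applies sword damage to the hit actor without checking the trace result.
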(event `InputAction|Attack`
  (params (Key :type "Key Structure"))
  (:`Pressed`
    (`self.Attack`)))

(event `Attack`
  (`self.MacroAttack`
    (:`YesMacro`
      (set `self.IsAttack` true)
      (`self.AttackEffects`))))

(event `AttackEffects`
  (bind _returnvalue (`self.PlayAnimMontage` "/Game/Player/Characters/ExtendedY-bot/Animations/AM_Attck.AM_Attck" (`self.AttackSpeed`)))
  (`KismetSystemLibrary.Delay` (/ _returnvalue (`self.AttackSpeed`)))
  (set `self.IsAttack` false))

(event `LaunchAttack`
  (bind _returnvalue (`self.K2_GetActorLocation`))
  (bind _outhit (`KismetSystemLibrary.LineTraceSingleForObjects` :`Start` _returnvalue :`End` (+ _returnvalue (* (`self.GetActorForwardVector`) (`self.AttackDistance`))) :`ObjectTypes` (`|MakeArray` "ObjectTypeQuery3" :!type "EObjectTypeQuery Enum") :`DrawDebugType` "ForDuration"))
  (if true
    (`GameplayStatics.ApplyDamage` (`.HitActor` (`GameplayStatics.BreakHitResult` _outhit)) (`self.Get Sword Damage`))))

(fn `Get Sword Damage`
  (returns (Damage :type "Float (double-precision)"))
  (return (`self.BaseDamage`)))

(fn `UserConstructionScript`
  (`parent.UserConstructionScript`))